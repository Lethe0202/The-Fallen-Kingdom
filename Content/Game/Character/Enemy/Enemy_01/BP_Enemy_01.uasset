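; Enemy character Blueprint that reports to player objectives when destroyed and shows its current action state as floating text.
; BeginPlay binds a handler to OnDestroyed, which passes the enemy's CharacterID to the PlayerCharacter's CallOnWorkObjectiveID, then calls DestroyActor after a delay.
; Every Tick, the TextRender displays the ActionComponent's current state and rotates to face the player camera.
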(event Custom|커스텀이벤트
  (params (DestroyedActor :type Actor%20Object%20Reference))
  (bind _asplayer_character (Utilities|Casting|CastToPlayerCharacter (Game|GetPlayerCharacter 0)))
  (Default|CallOnWorkObjectiveID _asplayer_character (Variables|Default|GetCharacterID))
  (Utilities|FlowControl|Delay 5.0)
  (Actor|DestroyActor))

(event EventBeginPlay
  (Game|BindEventtoOnDestroyed (delegate Custom|커스텀이벤트)))

(event Collision|EventActorBeginOverlap
  (params (OtherActor :type Actor%20Object%20Reference)))

(event EventTick
  (params (DeltaSeconds :type Float%20%28single-precision%29))
  (Rendering|Components|TextRender|SetText (Variables|Default|GetTextRender) (Utilities|Text|ToText(String) (Class|ActionComponent|GetCurrentStatetoString (Variables|Default|GetActionComponent))))
  (Transformation|SetWorldRotation (Variables|Default|GetTextRender) (Math|Rotator|FindLookatRotation (Transformation|GetActorLocation self) (Camera|GetCameraLocation (Game|GetPlayerCameraManager 0))) false false))

(fn ConstructionScript)