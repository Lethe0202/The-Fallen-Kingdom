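; Player controller that adds a debug panel to the screen and publishes the player character's transform data to materials.
; On BeginPlay it creates BP_DebugPanel for player 0 and adds it to the viewport.
; Every Tick it writes the character's location and yaw into the MPC_Player material parameter collection, setting the yaw parameter twice.
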(event EventBeginPlay
  (bind _returnvalue (UserInterface|CreateWidget "/Game/Game/UI/Debug/BP_DebugPanel.BP_DebugPanel_C" (Game|GetPlayerController 0)))
  (UserInterface|Viewport|AddtoViewport _returnvalue 0))

(event EventTick
  (params (DeltaSeconds :type Float%20%28single-precision%29))
  (Rendering|Material|SetScalarParameterValue "/Game/Game/UI/Map/MPC_Player.MPC_Player" "Player Yaw" (.yaw (Transformation|GetActorRotation (Game|GetPlayerCharacter 0))) :!class /Script/Engine.KismetMaterialLibrary)
  (Rendering|Material|SetVectorParameterValue "/Game/Game/UI/Map/MPC_Player.MPC_Player" "Player Location" (Math|Conversions|ToLinearColor(Vector) (Transformation|GetActorLocation (Game|GetPlayerCharacter 0))) :!class /Script/Engine.KismetMaterialLibrary)
  (Rendering|Material|SetScalarParameterValue "/Game/Game/UI/Map/MPC_Player.MPC_Player" "Player Yaw" (.Yaw (Math|Rotator|BreakRotator (Transformation|GetActorRotation (Game|GetPlayerCharacter 0)))) :!class /Script/Engine.KismetMaterialLibrary))

(fn ConstructionScript)