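; Player ability actor that acts as a slash damage-over-time area, judging by its name.
; From BeginPlay, a looping half-second timer runs a sphere trace for Pawns at the actor's root.
; Each hit actor is passed to CallOnExecuteEffectTarget, so the effect itself is applied outside this graph.
; The debug sphere draw is disconnected, and the graph has no logic to end the timer or destroy the actor.
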(event Custom|커스텀이벤트
  (bind _defaultsceneroot (Variables|Default|GetDefaultSceneRoot))
  (bind _returnvalue (Transformation|GetWorldLocation _defaultsceneroot))
  (bind (_outhits _returnvalue_2) (Collision|MultiSphereTraceForObjects _returnvalue _returnvalue 1e+02 (Utilities|Array|MakeArray "ObjectTypeQuery3") false 0 "None"))
  (if _returnvalue_2
    (for _array_element _outhits
      (Default|CallOnExecuteEffectTarget (.HitActor (Collision|BreakHitResult _array_element))))))

(event EventBeginPlay
  (Utilities|Time|SetTimerbyEvent (delegate Custom|커스텀이벤트) 0.5 true))

(event EventTick
  (params (DeltaSeconds :type Float%20%28single-precision%29)))

(fn ConstructionScript)