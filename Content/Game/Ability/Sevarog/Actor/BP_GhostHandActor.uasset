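; Sevarog ability actor that telegraphs a ghost hand attack with a filling decal, then strikes a box area.
; On BeginPlay, a timeline drives the decal material's Fill parameter.
; When it finishes, it hides the decal, swaps particle systems, box-traces ahead with a debug box, and broadcasts OnExecuteEffectTarget for each hit actor.
; The actor destroys itself when the second particle system finishes.
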(event Custom|OnSystemFinished_이벤트
  (params (PSystem :type Particle%20System%20Component%20Object%20Reference))
  (Actor|DestroyActor self))

(event EventBeginPlay
  (bind _particlesystem (Variables|Default|GetParticleSystem))
  (bind _particlesystem_2 (Variables|Default|GetParticleSystem))
  (bind _decal (Variables|Default|GetDecal))
  (bind _particlesystem1 (Variables|Default|GetParticleSystem1))
  (bind _returnvalue (Transformation|GetWorldLocation _particlesystem_2))
  (bind _returnvalue_2 (Math|Vector|GetForwardVector _particlesystem))
  (bind _returnvalue_3 (* _returnvalue_2 2.3e+02))
  (bind _returnvalue_4 (+ _returnvalue _returnvalue_3))
  ;[1 1 1 1 32] Attack Decal
  (bind _returnvalue_5 (Rendering|Material|CreateDynamicMaterialInstance (Variables|/Script/Engine.DecalComponent|GetDecalMaterial _decal) "None" "None" :!class /Script/Engine.KismetMaterialLibrary))
  (Rendering|Components|Decal|SetDecalMaterial _decal _returnvalue_5)
  (bind _새_트랙_0 (Timeline|타임라인 Play)
    (:Update
      (Rendering|Material|SetScalarParameterValue _returnvalue_5 "Fill" _새_트랙_0 :!class /Script/Engine.MaterialInstanceDynamic))
    (:Finished
      (Rendering|SetVisibility _decal false false)
      (Components|Activation|SetActive (Variables|Default|GetParticleSystem) false false)
      (Components|Activation|SetActive _particlesystem1 true false)
      (EventDispatchers|AssignOnSystemFinished _particlesystem1 (delegate Custom|OnSystemFinished_이벤트))
      (bind (_outhits _returnvalue_6) (Class|KismetSystemLibrary|BoxTraceMultiforObjects _returnvalue_4 _returnvalue_4 "100.000000,100.000000,100.000000" "0, 0, 0" (Variables|Default|GetObject%20Types) false 0 "None" true))
      (Class|QVSystemLibrary|DrawDebugBox _returnvalue_4 "100.000000,100.000000,100.000000" "(R=1.000000,G=0.000000,B=0.000000,A=1.000000)" "0, 0, 0" 5.0 0.0)
      (if _returnvalue_6
        (for _array_element _outhits
          (Default|CallOnExecuteEffectTarget (.HitActor (Collision|BreakHitResult _array_element))))))))

(event Collision|EventActorBeginOverlap
  (params (OtherActor :type Actor%20Object%20Reference)))

(fn ConstructionScript)