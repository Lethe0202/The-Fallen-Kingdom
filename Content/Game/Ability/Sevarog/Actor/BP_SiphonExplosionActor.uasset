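; Delayed area-of-effect explosion actor for Sevarog's Siphon ability, with a telegraphed ground decal.
; On BeginPlay a timeline animates the decal material's Fill parameter, hiding the decal when finished.
; In parallel, timed delays trigger the explosion particle, then a sphere trace that calls OnExecuteEffectTarget for each hit actor.
; A debug sphere draws at the trace location, and the actor destroys itself when the explosion particle finishes.
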(event OnSystemFinished(ParticleSystem1)
  (params (PSystem :type Particle%20System%20Component%20Object%20Reference))
  (Actor|DestroyActor))

(event EventBeginPlay
  (bind _particlesystem (Variables|Default|GetParticleSystem))
  (bind _particlesystem_2 (Variables|Default|GetParticleSystem))
  (bind _decal (Variables|Default|GetDecal))
  (bind _returnvalue (Transformation|GetWorldLocation _particlesystem_2))
  (bind _returnvalue_2 (Math|Vector|GetForwardVector _particlesystem))
  (bind _returnvalue_3 (* _returnvalue_2 ""))
  (bind _returnvalue_4 (+ _returnvalue _returnvalue_3))
  (Utilities|FlowControl|Sequence
    (:then_0
      ;[1 1 1 1 32] AttackDecal
      (bind _returnvalue_5 (Rendering|Material|CreateDynamicMaterialInstance (Variables|/Script/Engine.DecalComponent|GetDecalMaterial _decal) "None" "None" :!class /Script/Engine.KismetMaterialLibrary))
      (Rendering|Components|Decal|SetDecalMaterial _decal _returnvalue_5)
      (bind _새_트랙_1 (Timeline|타임라인 Play)
        (:Update
          (Rendering|Material|SetScalarParameterValue _returnvalue_5 "Fill" _새_트랙_1 :!class /Script/Engine.MaterialInstanceDynamic))
        (:Finished
          (Rendering|SetVisibility _decal false false))))
    (:then_1
      (Utilities|FlowControl|Delay 2.5)
      (Components|Activation|Activate (Variables|Default|GetParticleSystem1) false)
      (Utilities|FlowControl|Delay 0.5)
      (Components|Activation|Deactivate (Variables|Default|GetParticleSystem))
      (bind _outhits (Collision|MultiSphereTraceForObjects _returnvalue_4 _returnvalue_4 2.5e+02 (Variables|Default|GetObject%20Types) false 0 "None"))
      (Class|QVSystemLibrary|DrawDebugSphere _returnvalue_4 2.5e+02 12 "(R=1.000000,G=0.000000,B=0.000000,A=1.000000)" 5.0 0.0)
      (for _array_element _outhits
        (Default|CallOnExecuteEffectTarget (.HitActor (Collision|BreakHitResult _array_element)))))))

(event Collision|EventActorBeginOverlap
  (params (OtherActor :type Actor%20Object%20Reference)))

(fn ConstructionScript)