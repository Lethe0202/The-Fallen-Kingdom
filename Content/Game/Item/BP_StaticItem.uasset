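; BP_StaticItem is a placed or dropped pickup item that adds itself to the player's inventory when clicked.
; On BeginPlay, InitDropItem looks up ItemID in DT_ConsumptionItem to set the W_ItemInteractor widget's name text and blocking-load the static mesh.
; It also binds the widget's button, whose click calls AddItem on player 0's InventoryComponent and destroys the actor if that component exists.
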(event Custom|OnClicked_이벤트
  (bind _returnvalue (Game|GetPlayerCharacter 0))
  (bind _returnvalue_2 (Actor|GetComponentbyClass _returnvalue "/Script/QuarterViewGame.InventoryComponent"))
  (if (Utilities|IsValid _returnvalue_2)
    (Class|InventoryComponent|AddItem _returnvalue_2 (Utilities|String|ToString(Name) (Variables|Default|GetItemID)))
    (Actor|DestroyActor)))

(event Collision|EventActorBeginOverlap
  (params (OtherActor :type Actor%20Object%20Reference)))

(event EventTick
  (params (DeltaSeconds :type Float%20%28single-precision%29)))

(event EventInitDropItem
  (params (InItemID :type Name%20%28by%20ref%29 :default "None"))
  (|CallParentFunction InItemID)
  (Utilities|FlowControl|Sequence
    (:then_0
      (bind _asw_item_interactor (Utilities|Casting|CastToW_ItemInteractor (UserInterface|GetWidget (Variables|Default|GetWidget))))
      (EventDispatchers|AssignOnClicked (Variables|/Game/Game/UI/Item/W_ItemInteractor.W_ItemInteractor_C|GetButton_56 _asw_item_interactor) (delegate Custom|OnClicked_이벤트)))
    (:then_1
      (bind _returnvalue (Utilities|GetDataTableRow "/Game/Game/DataTable/Item/DT_ConsumptionItem.DT_ConsumptionItem" (Variables|Default|GetItemID))
        (:then
          (bind _asw_item_interactor_2 (Utilities|Casting|CastToW_ItemInteractor (UserInterface|GetWidget (Variables|Default|GetWidget))))
          (Variables|/Script/UMG.TextBlock|SetText (Variables|/Game/Game/UI/Item/W_ItemInteractor.W_ItemInteractor_C|GetDisplayName_Text _asw_item_interactor_2) (.DisplayName (Utilities|Struct|BreakConsumptionItemRow _returnvalue)))
          (bind _returnvalue_2 (Utilities|LoadAssetBlocking (.StaticMesh (Utilities|Struct|BreakConsumptionItemRow _returnvalue))))
          (bind _as스태틱_메시 (Utilities|Casting|CastToStaticMesh _returnvalue_2))
          (Components|StaticMesh|SetStaticMesh (Variables|Default|GetStaticMesh) _as스태틱_메시))))))

(event EventBeginPlay
  (Class|DropStaticItem|InitDropItem (Variables|Default|GetItemID)))

(fn ConstructionScript)