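; BP_LevelChangeVolume is an interactable portal that sends the player to another level.
; Its Box overlap events show a hidden Widget while the player character is inside and hide it again on exit.
; When the player interacts, it passes its Level and Options to ChangeLevel on the QuarterViewGameInstance.
; It also reports itself as a static Portal icon for the map.
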(event OnComponentBeginOverlap(Box)
  (params (OverlappedComponent :type Primitive%20Component%20Object%20Reference) (OtherActor :type Actor%20Object%20Reference) (OtherComp :type Primitive%20Component%20Object%20Reference) (OtherBodyIndex :type Integer) (bFromSweep :type Boolean) (SweepResult :type Hit%20Result%20Structure%20%28by%20ref%29))
  (if (== OtherActor (Game|GetPlayerCharacter 0))
    (Rendering|SetVisibility (Variables|Default|GetWidget) true false)))

(event OnComponentEndOverlap(Box)
  (params (OverlappedComponent :type Primitive%20Component%20Object%20Reference) (OtherActor :type Actor%20Object%20Reference) (OtherComp :type Primitive%20Component%20Object%20Reference) (OtherBodyIndex :type Integer))
  (if (== (Game|GetPlayerCharacter 0) OtherActor)
    (Rendering|SetVisibility (Variables|Default|GetWidget) false false)))

(event EventBeginPlay
  (Rendering|SetVisibility (Variables|Default|GetWidget) false false))

(event Collision|EventActorBeginOverlap
  (params (OtherActor :type Actor%20Object%20Reference)))

(event EventTick
  (params (DeltaSeconds :type Float%20%28single-precision%29)))

(event EventInteract
  (params (Interactor :type Actor%20Object%20Reference))
  (if (== Interactor (Game|GetPlayerCharacter 0))
    (bind _asquarter_view_game_instance (Utilities|Casting|CastToQuarterViewGameInstance (Game|GetGameInstance)))
    (Class|QuarterViewGameInstance|ChangeLevel _asquarter_view_game_instance (Variables|Default|GetLevel) (Variables|Default|GetOptions))))

(fn ConstructionScript)

(fn GetMapIconMovableType
  (return "Static"))

(fn GetMapIconType
  (return "Portal"))