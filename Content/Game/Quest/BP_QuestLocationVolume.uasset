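; Quest location volume that reports arrivals to the quest system and identifies itself as a static QuestLocation map icon.
; When any actor begins overlapping its sphere, it gets the quest manager from QuarterViewGameInstance and notifies it of one unit of progress for its LocationID, passing along that actor.
; The Blueprint does no actor filtering of its own, and its logic to hide the sphere and decal in game is disconnected.
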(event OnComponentBeginOverlap(SphereComponent)
  (params (OverlappedComponent :type Primitive%20Component%20Object%20Reference) (OtherActor :type Actor%20Object%20Reference) (OtherComp :type Primitive%20Component%20Object%20Reference) (OtherBodyIndex :type Integer) (bFromSweep :type Boolean) (SweepResult :type Hit%20Result%20Structure%20%28by%20ref%29))
  (bind _asquarter_view_game_instance (Utilities|Casting|CastToQuarterViewGameInstance (Game|GetGameInstance)))
  (Class|QuestManager|NotifyQuestQuantity (Class|QuarterViewGameInstance|GetQuestManager _asquarter_view_game_instance) OtherActor (Variables|Default|GetLocationID) 1))

(event EventBeginPlay)

(event Collision|EventActorBeginOverlap
  (params (OtherActor :type Actor%20Object%20Reference)))

(event EventTick
  (params (DeltaSeconds :type Float%20%28single-precision%29)))

(fn ConstructionScript)

(fn GetMapIconMovableType
  (return "Static"))

(fn GetMapIconType
  (return "QuestLocation"))